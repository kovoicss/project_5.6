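; BP_CoffeeMachine is an interactable coffee machine that turns coffee beans into coffee for a carried cup.
; Box overlap registers it in the first-person character's Interactibles list while nearby, and destroys any carried BP_CoffeeBean to increment BeanCount.
; Trigger sets IsCoffeeReady when beans exist; once ready, later triggers mark a held BP_Cup as holding coffee.
; BeanCount is never decremented and IsCoffeeReady is never reset here.
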(event `self.Box.OnComponentBeginOverlap`
  (params (OverlappedComponent :type "PrimitiveComponent Object Reference") (OtherActor :type "Actor Object Reference") (OtherComp :type "PrimitiveComponent Object Reference") (OtherBodyIndex :type Integer) (bFromSweep :type Boolean) (SweepResult :type "HitResult Structure (by ref)"))
  (bind _player (`self.Player`))
  (bind _asbp_first_person_character (cast `/Game/FirstPerson/Blueprints/BP_FirstPersonCharacter` OtherActor))
  (set `self.Player` _asbp_first_person_character)
  ; Add coffee machine to the interactible list for future use
  (`BlueprintSetLibrary.Set_Add` (`/Game/FirstPerson/Blueprints/BP_FirstPersonCharacter.Interactibles` _player) self)
  ; 咖啡豆相关逻辑
  (cast `/Game/Css/Blueprints/BP_CoffeeBean` (`/Game/FirstPerson/Blueprints/BP_FirstPersonCharacter.PickedUp` _player))
  (`self.K2_DestroyActor` (`/Game/FirstPerson/Blueprints/BP_FirstPersonCharacter.PickedUp` _asbp_first_person_character))
  (set `/Game/FirstPerson/Blueprints/BP_FirstPersonCharacter.PickedUp` null _asbp_first_person_character)
  (set `self.BeanCount` (+ (`self.BeanCount`) 1)))

(event `self.Box.OnComponentEndOverlap`
  (params (OverlappedComponent :type "PrimitiveComponent Object Reference") (OtherActor :type "Actor Object Reference") (OtherComp :type "PrimitiveComponent Object Reference") (OtherBodyIndex :type Integer))
  (cast `/Game/FirstPerson/Blueprints/BP_FirstPersonCharacter` OtherActor)
  ; Rmove coffee machine from the interactibles to avoid remote control
  (`BlueprintSetLibrary.Set_Remove` (`/Game/FirstPerson/Blueprints/BP_FirstPersonCharacter.Interactibles` (`self.Player`)) self)
  (set `self.Player` null))

(fn `Trigger`
  (returns (result :type Boolean))
  (if (`self.IsCoffeeReady`)
    (`/Engine/EditorBlueprintResources/StandardMacros.IsValid` (`self.Player`)
      (:`Is Valid`
        (bind _asbp_cup (cast `/Game/Css/Blueprints/BP_Cup` (`/Game/FirstPerson/Blueprints/BP_FirstPersonCharacter.PickedUp` (`self.Player`))))
        (set `/Game/Css/Blueprints/BP_Cup.IsHoldingCoffee` true _asbp_cup)
        (`KismetSystemLibrary.PrintString` "holding coffee"))
      (:`Is Not Valid`
        (`KismetSystemLibrary.PrintString` "Player is not next to Coffee machine but we attempted to interact; probably a bug")))
    (elif (> (`self.BeanCount`) 0)
      (`KismetSystemLibrary.PrintString` "Make Coffee")
      (set `self.IsCoffeeReady` true)
      (else
        (`KismetSystemLibrary.PrintString` "Not Enough Coffee bean"))))
  (return false))

(fn `UserConstructionScript`)