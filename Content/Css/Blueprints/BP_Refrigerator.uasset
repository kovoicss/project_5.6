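; BP_Refrigerator is an interactable food dispenser that gives the player packaged food from a limited stock.
; Trigger requires a valid Player with empty hands and a positive StorageCount, then spawns BP_PackagedFood, passes it to the player's Pickup and decrements the count.
; It returns false only when Player is invalid; full hands or empty storage just print a debug message and return true.
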(fn `Trigger`
  (returns (result :type Boolean))
  (bind _player (`self.Player`))
  (`/Engine/EditorBlueprintResources/StandardMacros.IsValid` _player
    (:`Is Valid`
      (`/Engine/EditorBlueprintResources/StandardMacros.IsValid` (`/Game/FirstPerson/Blueprints/BP_FirstPersonCharacter.PickedUp` _player)
        (:`Is Valid`
          (`KismetSystemLibrary.PrintString` "Player is already holding something; skipping interact")
          (return true))
        (:`Is Not Valid`
          (if (> (`self.StorageCount`) 0)
            (bind _returnvalue (`|SpawnActorFromClass` "/Game/Css/Blueprints/BP_PackagedFood.BP_PackagedFood_C" (`KismetMathLibrary.MakeTransform` (0.0 0.0 0.0)) "AlwaysSpawn" "MultiplyWithRoot" null null))
            (`/Game/FirstPerson/Blueprints/BP_FirstPersonCharacter.Pickup` _player _returnvalue)
            (`KismetSystemLibrary.PrintString` "Refrigerator pickup food")
            (set `self.StorageCount` (- (`self.StorageCount`) 1))
            (return true)
            (else
              (`KismetSystemLibrary.PrintString` "storage exhausted")
              (return true))))))
    (:`Is Not Valid`
      (return false))))

(fn `UserConstructionScript`)