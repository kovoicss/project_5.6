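; BP_Basin is an interactable basin where the player washes their hands or fills a watering can.
; It builds on a parent interactable that handles overlap, and binds a BeforeTrigger event that, with empty hands, plays audio and locks player input for the washing time.
; Trigger completes a GameMode task when hands are empty, fills a held BP_WateringCan, or rejects any other held item with a printed message.
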(event `Before Trigger`
  (`/Engine/EditorBlueprintResources/StandardMacros.IsValid` (`/Game/FirstPerson/Blueprints/BP_FirstPersonCharacter.PickedUp` (`self.Player`))
    (:`Is Not Valid`
      (`KismetSystemLibrary.PrintString` "Start Before Trigger")
      (`AudioComponent.Play` (`self.Audio`) 0.0)
      (`self.DisableInput` (`self.PlayerActor`) (`self.PlayerController`))
      (`KismetSystemLibrary.Delay` (`self.WashingTime`))
      (`self.EnableInput` (`self.PlayerActor`) (`self.PlayerController`))
      (`AudioComponent.Stop` (`self.Audio`)))))

(event `self.ReceiveBeginPlay`
  (`self.BeginPlayActual`)
  (add `self.BeforeTrigger` (delegate `Before Trigger`)))

(event `self.Box.OnComponentBeginOverlap`
  (params (OverlappedComponent :type "PrimitiveComponent Object Reference") (OtherActor :type "Actor Object Reference") (OtherComp :type "PrimitiveComponent Object Reference") (OtherBodyIndex :type Integer) (bFromSweep :type Boolean) (SweepResult :type "HitResult Structure (by ref)"))
  (`self.BeginOverlap` OtherActor))

(event `self.Box.OnComponentEndOverlap`
  (params (OverlappedComponent :type "PrimitiveComponent Object Reference") (OtherActor :type "Actor Object Reference") (OtherComp :type "PrimitiveComponent Object Reference") (OtherBodyIndex :type Integer))
  (`self.EndOverlap` OtherActor))

(fn `BeginOverlap`
  (params (actor :type "Actor Object Reference"))
  (`parent.BeginOverlap` actor))

(fn `BeginPlayActual`
  (`parent.BeginPlayActual`)
  (set `self.PlayerActor` (`GameplayStatics.GetPlayerPawn` 0))
  (set `self.PlayerController` (`GameplayStatics.GetPlayerController` 0)))

(fn `EndOverlap`
  (params (actor :type "Actor Object Reference"))
  (`parent.EndOverlap` actor))

(fn `Trigger`
  (returns (result :type Boolean))
  (bind _pickedup (`/Game/FirstPerson/Blueprints/BP_FirstPersonCharacter.PickedUp` (`self.Player`)))
  (`/Engine/EditorBlueprintResources/StandardMacros.IsValid` _pickedup
    (:`Is Valid`
      (bind _asbp_watering_can (cast `/Game/Css/Blueprints/BP_WateringCan` _pickedup)
        (:`then`
          (`/Game/Css/Blueprints/BP_WateringCan.GetWater` _asbp_watering_can)
          (return true))
        (:`CastFailed`
          (`KismetSystemLibrary.PrintString` "You cannot wash your hand with something in it")
          (return false))))
    (:`Is Not Valid`
      (`/Game/Css/Blueprints/BP_CSSGameMode.CompleteTask` (`self.GameMode`) 0)
      (return true))))

(fn `UserConstructionScript`)