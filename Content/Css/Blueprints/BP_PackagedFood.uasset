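; BP_PackagedFood is a food item the first-person character can pick up, drop and cook.
; A Box trigger registers the item as the character's Pickupable on overlap and clears it on exit.
; Pickup and drop extend the parent logic, switching the Box's collision and overlap events off while held and back on when dropped.
; Cook sets a cooked flag and swaps the mesh to a cooked material.
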(event `/Game/Css/Blueprints/Interfaces/BPI_Pickupable.drop`
  (`self.drop_actual`))

(event `/Game/Css/Blueprints/Interfaces/BPI_Pickupable.pickup`
  (`self.pickup_actual`))

(event `self.Box.OnComponentBeginOverlap`
  (params (OverlappedComponent :type "PrimitiveComponent Object Reference") (OtherActor :type "Actor Object Reference") (OtherComp :type "PrimitiveComponent Object Reference") (OtherBodyIndex :type Integer) (bFromSweep :type Boolean) (SweepResult :type "HitResult Structure (by ref)"))
  (bind _asbp_first_person_character (cast `/Game/Css/Blueprints/BP_FirstPersonCharacter` OtherActor))
  (set `/Game/Css/Blueprints/BP_FirstPersonCharacter.Pickupable` self _asbp_first_person_character)
  (`KismetSystemLibrary.PrintString` "In range"))

(event `self.Box.OnComponentEndOverlap`
  (params (OverlappedComponent :type "PrimitiveComponent Object Reference") (OtherActor :type "Actor Object Reference") (OtherComp :type "PrimitiveComponent Object Reference") (OtherBodyIndex :type Integer))
  (bind _asbp_first_person_character (cast `/Game/Css/Blueprints/BP_FirstPersonCharacter` OtherActor))
  (set `/Game/Css/Blueprints/BP_FirstPersonCharacter.Pickupable` null _asbp_first_person_character)
  (`KismetSystemLibrary.PrintString` "Out Of Range"))

(fn `Cook`
  (set `self.IsCooked` true)
  (`PrimitiveComponent.SetMaterial` (`self.StaticMesh`) 0 "/Game/Css/Materials/CookedFoodMaterial.CookedFoodMaterial"))

(fn `drop_actual`
  (bind _box (`self.Box`))
  (`parent.drop_actual`)
  (`KismetSystemLibrary.PrintString` "food dropped")
  (`PrimitiveComponent.SetCollisionResponseToAllChannels` _box "ECR_Overlap")
  (set `PrimitiveComponent.bGenerateOverlapEvents` true _box))

(fn `pickup_actual`
  (bind _box (`self.Box`))
  (`parent.pickup_actual`)
  (`KismetSystemLibrary.PrintString` "cup picked up")
  (`PrimitiveComponent.SetCollisionResponseToAllChannels` _box "ECR_Ignore")
  (set `PrimitiveComponent.bGenerateOverlapEvents` false _box))

(fn `UserConstructionScript`)