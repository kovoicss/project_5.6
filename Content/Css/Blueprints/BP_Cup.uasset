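; BP_Cup is a cup the first-person character can pick up and drop, extending a parent's pickup and drop logic.
; Entering its Box sets the character's Pickupable to the cup; clearing it on exit is disconnected.
; Pickup disables the Box's collision responses and overlap events, and drop restores them as overlaps.
; Highlight calls SetOverlayMaterial without a material, and debug prints trace the interactions.
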(event `/Game/Css/Blueprints/Interfaces/BPI_Pickupable.drop`
  (`self.drop_actual`))

(event `/Game/Css/Blueprints/Interfaces/BPI_Pickupable.pickup`
  (`self.pickup_actual`))

(event `self.Box.OnComponentBeginOverlap`
  (params (OverlappedComponent :type "PrimitiveComponent Object Reference") (OtherActor :type "Actor Object Reference") (OtherComp :type "PrimitiveComponent Object Reference") (OtherBodyIndex :type Integer) (bFromSweep :type Boolean) (SweepResult :type "HitResult Structure (by ref)"))
  (bind _asbp_first_person_character (cast `/Game/FirstPerson/Blueprints/BP_FirstPersonCharacter` OtherActor))
  (set `/Game/FirstPerson/Blueprints/BP_FirstPersonCharacter.Pickupable` self _asbp_first_person_character)
  (`KismetSystemLibrary.PrintString` "In range"))

(event `self.Box.OnComponentEndOverlap`
  (params (OverlappedComponent :type "PrimitiveComponent Object Reference") (OtherActor :type "Actor Object Reference") (OtherComp :type "PrimitiveComponent Object Reference") (OtherBodyIndex :type Integer)))

(event `/Game/Css/Blueprints/Interfaces/BPI_Pickupable.highlight`
  ;[0.15 0.03396 0.04386 0.5] Overlay material needs to be added
  (`MeshComponent.SetOverlayMaterial` (`self.StaticMesh`) null)
  (`KismetSystemLibrary.PrintString` "highlight"))

(fn `drop_actual`
  (bind _box (`self.Box`))
  (`parent.drop_actual`)
  (`KismetSystemLibrary.PrintString` "cup dropped")
  (`PrimitiveComponent.SetCollisionResponseToAllChannels` _box "ECR_Overlap")
  (set `PrimitiveComponent.bGenerateOverlapEvents` true _box))

(fn `pickup_actual`
  (bind _box (`self.Box`))
  (`parent.pickup_actual`)
  (`KismetSystemLibrary.PrintString` "cup picked up")
  (`PrimitiveComponent.SetCollisionResponseToAllChannels` _box "ECR_Ignore")
  (set `PrimitiveComponent.bGenerateOverlapEvents` false _box))

(fn `UserConstructionScript`)