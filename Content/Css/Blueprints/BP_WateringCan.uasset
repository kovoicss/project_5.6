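; BP_WateringCan is a watering can item that the first-person character can pick up and drop.
; Entering its Box registers the can as the character's Pickupable, and the Pickup and Drop events forward to PickupActual and DropActual.
; Leaving the Box does nothing, as the logic that clears Pickupable is disconnected.
; Water sets the Watering flag and swaps the mesh material to CookedFoodMaterial.
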(event `/Game/Css/Blueprints/Interfaces/BPI_Pickupable.drop`
  (`self.drop_actual`))

(event `/Game/Css/Blueprints/Interfaces/BPI_Pickupable.pickup`
  (`self.pickup_actual`))

(event `self.Box.OnComponentBeginOverlap`
  (params (OverlappedComponent :type "PrimitiveComponent Object Reference") (OtherActor :type "Actor Object Reference") (OtherComp :type "PrimitiveComponent Object Reference") (OtherBodyIndex :type Integer) (bFromSweep :type Boolean) (SweepResult :type "HitResult Structure (by ref)"))
  (bind _asbp_first_person_character (cast `/Game/FirstPerson/Blueprints/BP_FirstPersonCharacter` OtherActor))
  (set `/Game/FirstPerson/Blueprints/BP_FirstPersonCharacter.Pickupable` self _asbp_first_person_character)
  (`KismetSystemLibrary.PrintString` "In range"))

(event `self.Box.OnComponentEndOverlap`
  (params (OverlappedComponent :type "PrimitiveComponent Object Reference") (OtherActor :type "Actor Object Reference") (OtherComp :type "PrimitiveComponent Object Reference") (OtherBodyIndex :type Integer)))

(fn `UserConstructionScript`)

(fn `Water`
  (set `self.Watering` true)
  (`PrimitiveComponent.SetMaterial` (`self.StaticMesh`) 0 "/Game/Css/Materials/CookedFoodMaterial.CookedFoodMaterial"))