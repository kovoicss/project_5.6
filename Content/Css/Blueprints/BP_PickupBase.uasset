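; BP_PickupBase is a base Blueprint for objects that can be picked up and dropped, built around a StaticMesh.
; The Pickup and Drop events forward to the PickupActual and DropActual functions.
; Pickup turns off physics, gravity and collision on the mesh and prints a debug string.
; Drop restores simulated physics, gravity and full blocking collision.
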(event `/Game/Css/Blueprints/Interfaces/BPI_Pickupable.pickup`
  (`self.pickup_actual`))

(event `/Game/Css/Blueprints/Interfaces/BPI_Pickupable.drop`
  (`self.drop_actual`))

(fn `drop_actual`
  (bind _staticmesh (`self.StaticMesh`))
  (`PrimitiveComponent.SetSimulatePhysics` _staticmesh true)
  (`PrimitiveComponent.SetEnableGravity` _staticmesh true)
  (`PrimitiveComponent.SetCollisionEnabled` _staticmesh "QueryAndPhysics")
  (`PrimitiveComponent.SetCollisionResponseToAllChannels` _staticmesh "ECR_Block"))

(fn `pickup_actual`
  (bind _staticmesh (`self.StaticMesh`))
  (`PrimitiveComponent.SetSimulatePhysics` _staticmesh false)
  (`PrimitiveComponent.SetEnableGravity` _staticmesh false)
  (`PrimitiveComponent.SetCollisionEnabled` _staticmesh "NoCollision")
  (`PrimitiveComponent.SetCollisionResponseToAllChannels` _staticmesh "ECR_Ignore")
  (`KismetSystemLibrary.PrintString` "pickup base pickup_actual"))

(fn `UserConstructionScript`)