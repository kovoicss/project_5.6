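; BP_Flower is an interactable flower that the player waters with a carried BP_WateringCan to complete a GameMode task.
; CheckCanWater allows this only while the flower is unwatered and the held can contains water.
; A bound BeforeTrigger event plays audio and locks player input for the watering time, then swaps the mesh material.
; Trigger uses the can's water, marks the flower watered and reports the task complete.
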(event `Before Trigger`
  (bind _result (`self.CheckCanWater`))
  (if _result
    (`KismetSystemLibrary.PrintString` "Start Before Trigger")
    (`AudioComponent.Play` (`self.Audio`) 0.0)
    (`self.DisableInput` (`self.PlayerActor`) (`self.PlayerController`))
    (`KismetSystemLibrary.Delay` (`self.WateringTime`))
    (`self.EnableInput` (`self.PlayerActor`) (`self.PlayerController`))
    (`AudioComponent.Stop` (`self.Audio`))
    (`PrimitiveComponent.SetMaterial` (`self.StaticMesh`) 0 "/Game/Css/Materials/FlowerMaterial.FlowerMaterial")))

(event `self.ReceiveBeginPlay`
  (`self.BeginPlayActual`)
  (add `self.BeforeTrigger` (delegate `Before Trigger`)))

(fn `BeginOverlap`
  (params (actor :type "Actor Object Reference"))
  (`parent.BeginOverlap` actor))

(fn `BeginPlayActual`
  (`parent.BeginPlayActual`)
  (set `self.PlayerActor` (`GameplayStatics.GetPlayerPawn` 0))
  (set `self.PlayerController` (`GameplayStatics.GetPlayerController` 0)))

(fn `CheckCanWater`
  (returns (Result :type Boolean) (WaterCan :type "/Game/Css/Blueprints/BP_WateringCan Object Reference"))
  (bind _pickedup (`/Game/Css/Blueprints/BP_FirstPersonCharacter.PickedUp` (`self.Player`)))
  (if (not (`self.IsWatered`))
    (`/Engine/EditorBlueprintResources/StandardMacros.IsValid` _pickedup
      (:`Is Valid`
        (bind _asbp_watering_can (cast `/Game/Css/Blueprints/BP_WateringCan` _pickedup)
          (:`then`
            (return (`/Game/Css/Blueprints/BP_WateringCan.Is contain water` _asbp_watering_can) _asbp_watering_can))
          (:`CastFailed`
            _)))
      (:`Is Not Valid`
        _)))
  (return false null))

(fn `EndOverlap`
  (params (actor :type "Actor Object Reference"))
  (`parent.EndOverlap` actor))

(fn `Trigger`
  (returns (result :type Boolean))
  (bind (_result _watercan) (`self.CheckCanWater`))
  (if _result
    (`/Game/Css/Blueprints/BP_WateringCan.Water` _watercan)
    (set `self.IsWatered` true)
    (`/Game/Css/Blueprints/BP_CSSGameMode.CompleteTask` (`self.GameMode`) 5)
    (`KismetSystemLibrary.PrintString` "Flower Is Watered")
    (return true)
    (else
      (return false))))

(fn `UserConstructionScript`)

(fn `Watered`
  (set `self.IsWatered` true)
  (`PrimitiveComponent.SetMaterial` (`self.StaticMesh`) 0 "/Game/Css/Materials/CookedFoodMaterial.CookedFoodMaterial"))