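; BP_ClothBasket is a cloth basket that the first-person character can pick up and drop.
; Its Box overlap sets or clears the character's Pickupable reference and prints debug range messages.
; The Pickup and Drop events forward to PickupActual and DropActual, whose logic is not defined here.
; TakeCleanCloth flags the basket as containing cloth that is cleaned.
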(event `/Game/Css/Blueprints/Interfaces/BPI_Pickupable.pickup`
  (`self.pickup_actual`))

(event `/Game/Css/Blueprints/Interfaces/BPI_Pickupable.drop`
  (`self.drop_actual`))

(event `self.Box.OnComponentBeginOverlap`
  (params (OverlappedComponent :type "PrimitiveComponent Object Reference") (OtherActor :type "Actor Object Reference") (OtherComp :type "PrimitiveComponent Object Reference") (OtherBodyIndex :type Integer) (bFromSweep :type Boolean) (SweepResult :type "HitResult Structure (by ref)"))
  (bind _asbp_first_person_character (cast `/Game/Css/Blueprints/BP_FirstPersonCharacter` OtherActor))
  (set `/Game/Css/Blueprints/BP_FirstPersonCharacter.Pickupable` self _asbp_first_person_character)
  (`KismetSystemLibrary.PrintString` "In range"))

(event `self.Box.OnComponentEndOverlap`
  (params (OverlappedComponent :type "PrimitiveComponent Object Reference") (OtherActor :type "Actor Object Reference") (OtherComp :type "PrimitiveComponent Object Reference") (OtherBodyIndex :type Integer))
  (bind _asbp_first_person_character (cast `/Game/Css/Blueprints/BP_FirstPersonCharacter` OtherActor))
  (set `/Game/Css/Blueprints/BP_FirstPersonCharacter.Pickupable` null _asbp_first_person_character)
  (`KismetSystemLibrary.PrintString` "Out Of Range"))

(fn `TakeCleanCloth`
  (set `self.IsContainCloth` true)
  (set `self.IsClothCleaned` true))

(fn `UserConstructionScript`)