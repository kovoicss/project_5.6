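; BP_Note is an interactable note actor that opens and closes a note UI when triggered.
; On BeginPlay it caches the player controller and game mode and creates its own empty UI_Note widget.
; Trigger toggles viewing by adding that widget to the game mode's shared NoteUI, focusing its text box and switching the mouse cursor.
; Highlight and UnHighlight swap the mesh material, and FaceDirection sets the actor's rotation.
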(event `self.ReceiveBeginPlay`
  (`PrimitiveComponent.SetMaterial` (`self.StaticMesh1`) 0 (`self.NormalMaterial`))
  (set `self.PlayerActor` (`GameplayStatics.GetPlayerPawn` 0))
  (set `self.PlayerController` (`GameplayStatics.GetPlayerController` 0))
  (bind _asbp_cssgame_mode (cast `/Game/Css/Blueprints/BP_CSSGameMode` (`GameplayStatics.GetGameMode`)))
  (set `self.GameMode` _asbp_cssgame_mode)
  (bind _returnvalue (`|CreateWidget` "/Game/UI/UI_Note.UI_Note_C"))
  (bind _output_get (set `self.UI_Note` _returnvalue))
  (set `/Game/UI/UI_Note.NoteText` "" _output_get))

(fn `BeginPlayActual`)

(fn `FaceDirection`
  (params (rotation :type "Rotator Structure"))
  (`self.K2_SetActorRotation` rotation))

(fn `Highlight`
  (`PrimitiveComponent.SetMaterial` (`self.StaticMesh1`) 0 (`self.HighlightMaterial`)))

(fn `Trigger`
  (returns (result :type Boolean))
  (bind _playercontroller (`self.PlayerController`))
  (bind _ui_note (`self.UI_Note`))
  (bind _noteui (`/Game/Css/Blueprints/BP_CSSGameMode.NoteUI` (`self.GameMode`)))
  (if (`self.IsViewing`)
    (`Widget.RemoveFromParent` _noteui)
    (set `PlayerController.bShowMouseCursor` false _playercontroller)
    (set `self.IsViewing` false)
    (else
      (`/Game/UI/UI_NoteMenu.AddNote` _noteui _ui_note)
      (`UserWidget.AddToPlayerScreen` _noteui 0)
      (`Widget.SetFocus` (`/Game/UI/UI_Note.NoteTextBox` _ui_note))
      (set `PlayerController.bShowMouseCursor` true _playercontroller)
      (set `self.IsViewing` true)))
  (return true))

(fn `UnHighlight`
  (`PrimitiveComponent.SetMaterial` (`self.StaticMesh1`) 0 (`self.NormalMaterial`))
  (`KismetSystemLibrary.PrintString` "Hello"))

(fn `UserConstructionScript`)