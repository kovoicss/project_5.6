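; BP_CSSGameMode is a game mode that drives the player's task list and owns the main game UI.
; On BeginPlay it finds the level's BP_TaskManager, adds the game HUD to the viewport and creates a note menu widget without showing it.
; CompleteTask and GenerateTaskList forward to the task manager, then RefreshHUD rebuilds the HUD list with one task widget per current task, named from TaskMap.
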(event `self.ReceiveBeginPlay`
  (bind _returnvalue (`GameplayStatics.GetActorOfClass` "/Game/Css/Blueprints/BP_TaskManager.BP_TaskManager_C"))
  (set `self.TaskManager` _returnvalue)
  (bind _returnvalue_2 (`|CreateWidget` "/Game/UI/UI_GameHUD.UI_GameHUD_C"))
  (`UserWidget.AddToViewport` _returnvalue_2 0)
  (set `self.HUD` _returnvalue_2)
  (`self.RefreshHUD`)
  (bind _returnvalue_3 (`|CreateWidget` "/Game/UI/UI_NoteMenu.UI_NoteMenu_C"))
  (set `self.NoteUI` _returnvalue_3))

(fn `CompleteTask`
  (params (TaskNum :type Integer))
  (`/Game/Css/Blueprints/BP_TaskManager.CompleteTask` (`self.TaskManager`) TaskNum)
  (`self.RefreshHUD`))

(fn `GenerateTaskList`
  (`/Game/Css/Blueprints/BP_TaskManager.GenerateTaskList` (`self.TaskManager`))
  (`self.RefreshHUD`))

(fn `RefreshHUD`
  (bind _taskmanager (`self.TaskManager`))
  (`/Game/UI/UI_Tasklist.ClearTaskList` (`/Game/UI/UI_GameHUD.UI_Tasklist` (`self.HUD`)))
  (bind _result (`BlueprintSetLibrary.Set_ToArray` (`/Game/Css/Blueprints/BP_TaskManager.CurrentTask` _taskmanager)))
  (for _array_element _result
    (bind _returnvalue (`|CreateWidget` "/Game/UI/UI_Task.UI_Task_C"))
    (set `/Game/UI/UI_Task.Name` (`.UI_name_7_A1DE17D445AE9908ADB2E88BE633250B` (break `/Game/Css/Blueprints/Task` (`BlueprintMapLibrary.Map_Find` (`/Game/Css/Blueprints/BP_TaskManager.TaskMap` _taskmanager) _array_element))) _returnvalue)
    (`/Game/UI/UI_Tasklist.AddTaskToList` (`/Game/UI/UI_GameHUD.UI_Tasklist` (`self.HUD`)) _returnvalue)))

(fn `UserConstructionScript`)