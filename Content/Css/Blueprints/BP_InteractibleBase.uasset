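; Base Blueprint for interactible objects that the first-person character can use while standing in range.
; Box overlap events add the object to the character's Interactibles list and cache that Player, then remove it and clear the reference on exit, preventing remote use.
; Both transitions print a debug message.
; Trigger is a stub that returns false and holds no interaction logic.
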(event `self.Box.OnComponentBeginOverlap`
  (params (OverlappedComponent :type "PrimitiveComponent Object Reference") (OtherActor :type "Actor Object Reference") (OtherComp :type "PrimitiveComponent Object Reference") (OtherBodyIndex :type Integer) (bFromSweep :type Boolean) (SweepResult :type "HitResult Structure (by ref)"))
  (`self.BeginOverlap` OtherActor))

(event `self.Box.OnComponentEndOverlap`
  (params (OverlappedComponent :type "PrimitiveComponent Object Reference") (OtherActor :type "Actor Object Reference") (OtherComp :type "PrimitiveComponent Object Reference") (OtherBodyIndex :type Integer))
  (`self.EndOverlap` OtherActor))

(fn `BeginOverlap`
  (params (actor :type "Actor Object Reference"))
  (bind _asbp_first_person_character (cast `/Game/FirstPerson/Blueprints/BP_FirstPersonCharacter` actor))
  (set `self.Player` _asbp_first_person_character)
  ; Add coffee machine to the interactible list for future use
  (`BlueprintSetLibrary.Set_Add` (`/Game/FirstPerson/Blueprints/BP_FirstPersonCharacter.Interactibles` (`self.Player`)) self)
  (`KismetSystemLibrary.PrintString` "In range for interact"))

(fn `EndOverlap`
  (params (actor :type "Actor Object Reference"))
  (cast `/Game/FirstPerson/Blueprints/BP_FirstPersonCharacter` actor)
  ; Rmove coffee machine from the interactibles to avoid remote control
  (`BlueprintSetLibrary.Set_Remove` (`/Game/FirstPerson/Blueprints/BP_FirstPersonCharacter.Interactibles` (`self.Player`)) self)
  (set `self.Player` null)
  (`KismetSystemLibrary.PrintString` "Out of range for interact"))

(fn `Trigger`
  (returns (result :type Boolean))
  (return false))

(fn `UserConstructionScript`)