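; BP_WashingMachine is an interactable washing machine that runs a timed wash and hands clean cloth to the player's basket.
; Trigger requires a carried BP_ClothBasket, then either gives it clean cloth, refuses while running, or fires the StartWashing dispatcher.
; Its bound handler uses a DoOnce gate and FinishTime delay, then flags the cloth clean and plays audio.
; The text-facing LookAtPlayer function is unfinished and never runs.
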(event `self.ReceiveBeginPlay`
  (add `self.StartWashing` (delegate `CustomEvent`))
  (set `self.PlayerRef` (`GameplayStatics.GetPlayerPawn` 0)))

(event `CustomEvent`
  (`/Engine/EditorBlueprintResources/StandardMacros.DoOnce` false :!label _label
    (:`Completed`
      (set `self.IsRunning` true)
      (`KismetSystemLibrary.Delay` (`self.FinishTime`))
      (set `self.IsClothCleaned` true)
      (`AudioComponent.Play` (`self.Audio`) 0.0)
      (set `self.IsRunning` false)
      (goto _label :!via `Reset`))))

(event `self.ReceiveTick`
  (params (DeltaSeconds :type "Float (single-precision)")))

(fn `LookAtPlayer`
  (bind _textrender (`self.TextRender`))
  ;[0.15 0.0513 0.05201 0.5] TODO: Needs to be fixed
  (`SceneComponent.K2_SetWorldTransform` _textrender (`KismetAnimationLibrary.K2_LookAt` (`SceneComponent.K2_GetComponentToWorld` _textrender) (`self.K2_GetActorLocation` (`self.PlayerRef`))) false true))

(fn `Trigger`
  (returns (result :type Boolean))
  (bind _pickedup (`/Game/FirstPerson/Blueprints/BP_FirstPersonCharacter.PickedUp` (`self.Player`)))
  (`/Engine/EditorBlueprintResources/StandardMacros.IsValid` (`self.Player`)
    (:`Is Valid`
      (`/Engine/EditorBlueprintResources/StandardMacros.IsValid` _pickedup
        (:`Is Valid`
          (bind _asbp_cloth_basket (cast `/Game/Css/Blueprints/BP_ClothBasket` _pickedup)
            (:`then`
              (if (`self.IsClothCleaned`)
                (`/Game/Css/Blueprints/BP_ClothBasket.TakeCleanCloth` _asbp_cloth_basket)
                (`KismetSystemLibrary.PrintString` "Cleaned Cloth is taken")
                (return true)
                (elif (`self.IsRunning`)
                  (`KismetSystemLibrary.PrintString` "Washing machine is still running")
                  (return false)
                  (else
                    (`self.StartWashing`)
                    (return true)))))
            (:`CastFailed`
              _)))
        (:`Is Not Valid`
          _)))
    (:`Is Not Valid`
      _))
  (return false))

(fn `UserConstructionScript`)