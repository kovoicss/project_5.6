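; BP_door is a door Blueprint that alternates between open and closed each time it is triggered.
; Its trigger event calls TriggerDoor, which plays either the open or close sequence based on the IsOpen flag, then flips the flag.
; The door is flagged closed at BeginPlay, and a separate Trigger function only returns false.
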(event `self.ReceiveBeginPlay`
  (set `self.Is Open` false))

(event `Trigger_1_1`
  (`self.TriggerDoor`))

(fn `Trigger`
  (returns (result :type Boolean))
  (return false))

(fn `TriggerDoor`
  (if (`self.Is Open`)
    (`ActorSequenceComponent.PlaySequence` (`self.DoorCloseSequence`))
    (set `self.Is Open` false)
    (else
      (`ActorSequenceComponent.PlaySequence` (`self.DoorOpenSequence`))
      (set `self.Is Open` true))))

(fn `UserConstructionScript`)