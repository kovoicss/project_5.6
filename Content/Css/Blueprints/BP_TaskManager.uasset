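; BP_TaskManager tracks the player's household chores, such as washing hands and making coffee.
; BeginPlay builds TaskMap keyed by task number, fills in only the first two of ten entries, and marks those two as current.
; GetTask looks up a task by number, while CompleteTask removes it from CurrentTask and prints the number.
; CreateTaskList is an empty stub, and names for further chores sit unconnected in the graph.
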(event `self.ReceiveBeginPlay`
  (bind _currenttask (`self.CurrentTask`))
  (set `self.TaskMap` (`|MakeMap` 0 (make `/Game/Css/Blueprints/Task` "wash" "Wash your hands" 0) 1 (make `/Game/Css/Blueprints/Task` "make_coffee" "Make a cup of coffee" 1) 2 (struct) 3 (struct) 4 (struct) 5 (struct) 6 (struct) 7 (struct) 8 (struct) 9))
  (`BlueprintSetLibrary.Set_Add` _currenttask)
  (`BlueprintSetLibrary.Set_Add` _currenttask 1))

(fn `CompleteTask`
  (params (TaskNum :type Integer))
  (`BlueprintSetLibrary.Set_Remove` (`self.CurrentTask`) TaskNum)
  (`KismetSystemLibrary.PrintString` (`KismetStringLibrary.Conv_IntToString` TaskNum)))

(fn `CreateTaskList`
  (returns (task_list :type "Array of Integer"))
  (return))

(fn `GetTask`
  (params (TaskNum :type Integer))
  (returns (Task :type "/Game/Css/Blueprints/Task Structure"))
  (bind (_value _returnvalue) (`BlueprintMapLibrary.Map_Find` (`self.TaskMap`) TaskNum))
  (if _returnvalue
    (return _value)
    (else
      (return))))

(fn `UserConstructionScript`)