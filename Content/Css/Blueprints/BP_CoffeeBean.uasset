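; BP_CoffeeBean is a coffee bean item that the first-person character can pick up and drop.
; Overlapping its Box registers the bean as the character's Pickupable.
; Pickup and drop events call overrides that run the parent logic, then set the Box to ignore all channels while held and restore overlap on drop.
; Debug prints trace each step, though the drop message says "cup dropped".
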(event `pickup_1`
  (`self.pickup_actual`))

(event `drop_1`
  (`self.drop_actual`))

(event `self.Box.OnComponentBeginOverlap`
  (params (OverlappedComponent :type "PrimitiveComponent Object Reference") (OtherActor :type "Actor Object Reference") (OtherComp :type "PrimitiveComponent Object Reference") (OtherBodyIndex :type Integer) (bFromSweep :type Boolean) (SweepResult :type "HitResult Structure (by ref)"))
  (bind _asbp_first_person_character (cast `/Game/Css/Blueprints/BP_FirstPersonCharacter` OtherActor))
  (set `/Game/Css/Blueprints/BP_FirstPersonCharacter.Pickupable` self _asbp_first_person_character)
  (`KismetSystemLibrary.PrintString` "In Range"))

(fn `drop_actual`
  (bind _box (`self.Box`))
  (`parent.drop_actual`)
  (`KismetSystemLibrary.PrintString` "cup dropped")
  (`PrimitiveComponent.SetCollisionResponseToAllChannels` _box "ECR_Overlap")
  (set `PrimitiveComponent.bGenerateOverlapEvents` true _box))

(fn `pickup_actual`
  (`parent.pickup_actual`)
  (`KismetSystemLibrary.PrintString` "CoffeeBean Pickup")
  (`PrimitiveComponent.SetCollisionResponseToAllChannels` (`self.Box`) "ECR_Ignore"))

(fn `UserConstructionScript`)