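; BP_door is a door Blueprint that toggles between open and closed when its Trigger event fires.
; Trigger calls TriggerDoor, which checks the IsOpen flag, plays either the open or close sequence, and flips the flag.
; BeginPlay resets IsOpen to false, so the door starts closed.
; An unused FlipFlop version of the same toggle remains disconnected in TriggerDoor.
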(event `self.ReceiveBeginPlay`
  (set `self.Is Open` false))

(event `/Game/Css/BPI_Interactible.Trigger`
  (`self.TriggerDoor`))

(fn `TriggerDoor`
  (if (`self.Is Open`)
    (`ActorSequenceComponent.PlaySequence` (`self.DoorCloseSequence`))
    (set `self.Is Open` false)
    (else
      (`ActorSequenceComponent.PlaySequence` (`self.DoorOpenSequence`))
      (set `self.Is Open` true))))

(fn `UserConstructionScript`)